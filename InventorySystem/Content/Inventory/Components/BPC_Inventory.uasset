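; Player inventory component that stores swords, shields and eatables in resizable slot arrays, and also tracks money and health.
; A per-tick sphere trace drives the interact prompt, and Interact adds the item, stacking up to DT_Items limits before taking an empty slot.
; Money pickup reads DT_Money, while inventory and health changes push updates to their widgets.
; Debug keys test resizing and item decrement, which searches only swords and skips the UI refresh.
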(event EventBeginPlay
  (bind _allitem (Variables|Default|GetAllItem))
  (bind (_swords _shield _eatable) (Utilities|Struct|BreakS_AllItem _allitem))
  ;[1 1 1] Input mapping
  (Input|AddMappingContext (PlayerController|LocalPlayerSubsystems|GetEnhancedInputLocalPlayerSubsystem (Game|GetPlayerController 0)) "/Game/Inventory/Inputs/IMC_InventoryInput.IMC_InventoryInput" 0 "(bIgnoreAllPressedKeysUntilRelease=True,bForceImmediately=False,bNotifyUserSettings=False)")
  (bind _returnvalue (UserInterface|CreateWidget "/Game/Inventory/Widgets/WBP_Inventory.WBP_Inventory_C"))
  (Variables|Widget|SetWBP_Inventory _returnvalue)
  (bind _asbp_first_person_character (Utilities|Casting|CastToBP_FirstPersonCharacter (Game|GetPlayerCharacter 0)))
  (bind _output_get (Variables|Default|SetAs%20BP%20First%20Person%20Character _asbp_first_person_character))
  (Collision|BindEventtoOnComponentBeginOverlap (Variables|/Script/Engine.Character|GetCapsuleComponent _output_get) (EventDispatchers|CreateEvent :!event PickUpMoney))
  ;[1 1 1] Health bar in game play
  (HealthBar|HealthBarInitialization)
  ;[1 1 1] Create interact ui in gameplay
  (bind _returnvalue_2 (UserInterface|CreateWidget "/Game/Inventory/Widgets/WBP_Interact.WBP_Interact_C"))
  (Variables|Widget|SetWBP_Interact _returnvalue_2)
  ;[1 1 1] initial inventory size
  (Utilities|Array|Resize _swords 5)
  (Utilities|Array|Resize _shield 8)
  (Utilities|Array|Resize _eatable 7)
  (Default|UpdateItemsinInventoryUI (Variables|Widget|GetWBP_Inventory) (Variables|Default|GetAllItem)))

(event EventTick
  (params (DeltaSeconds :type Float%20%28single-precision%29))
  (bind _wbp_interact (Variables|Widget|GetWBP_Interact))
  (bind _wbp_interact_2 (Variables|Widget|GetWBP_Interact))
  (bind _wbp_iteminfo (Variables|/Game/Inventory/Widgets/WBP_Interact.WBP_Interact_C|GetWBP_ItemInfo _wbp_interact_2))
  ;[1 1 1] Trace item on Ray and update info
  (bind (_item _founditem) (Inventory|TraceItemtoPickUp))
  (Variables|/Game/Inventory/Widgets/WBP_ItemInfo.WBP_ItemInfo_C|SetItem _wbp_iteminfo _item)
  (Default|UpdateItemInfo _wbp_iteminfo)
  (if _founditem
    (UserInterface|Viewport|AddtoViewport _wbp_interact 0)
    (else
      (Widget|RemovefromParent _wbp_interact))))

(event Input|KeyboardEvents|N
  (params (Key :type Key%20Structure :default "None"))
  ;[1 1 1] Test
  (:Pressed
    (Inventory|SetInventorySize 8 3 3)))

(event Input|KeyboardEvents|M
  (params (Key :type Key%20Structure :default "None"))
  ;[1 1 1] Test
  (:Pressed
    (Inventory|UpgradeInventory 2 2 2)))

(event Input|KeyboardEvents|T
  (params (Key :type Key%20Structure :default "None"))
  (:Pressed
    (CallFunction|DecreaseQuantityOfSpecificItemName (Variables|Default|GetSpecificItem))))

(event Input|EnhancedActionEvents|EnhancedInputActionIA_Inventory
  (params (ActionValue :type Boolean) (ElapsedSeconds :type Float%20%28double-precision%29) (TriggeredSeconds :type Float%20%28double-precision%29) (InputAction :type Input%20Action%20Object%20Reference :default "/Game/Inventory/Inputs/IA_Inventory.IA_Inventory"))
  (bind _returnvalue (Game|GetPlayerController 0))
  ;[1 1 1] Add inventory widget to viewport
  (UserInterface|Viewport|AddtoViewport (Variables|Widget|GetWBP_Inventory) 0)
  (Variables|/Script/Engine.PlayerController|SetbShowMouseCursor _returnvalue true)
  (Input|SetInputModeUIOnly _returnvalue (Variables|Widget|GetWBP_Inventory) "DoNotLock" false)
  (Default|UpdateItemsinInventoryUI (Variables|Widget|GetWBP_Inventory) (Variables|Default|GetAllItem)))

(event Input|EnhancedActionEvents|EnhancedInputActionIA_Interact
  (params (ActionValue :type Boolean) (ElapsedSeconds :type Float%20%28double-precision%29) (TriggeredSeconds :type Float%20%28double-precision%29) (InputAction :type Input%20Action%20Object%20Reference :default "/Game/Inventory/Inputs/IA_Interact.IA_Interact"))
  (bind (_item _founditem _itemactor) (Inventory|TraceItemtoPickUp))
  (if _founditem
    (bind _success (Inventory|AddtoInventory _item))
    (if _success
      (Actor|DestroyActor _itemactor)
      (Default|UpdateItemsinInventoryUI (Variables|Widget|GetWBP_Inventory) (Variables|Default|GetAllItem))
      (else
        (Development|PrintString "Add to inventory fail")))))

(fn PickUpMoney
  (params (OverlappedComponent :type Primitive%20Component%20Object%20Reference) (OtherActor :type Actor%20Object%20Reference) (OtherComp :type Primitive%20Component%20Object%20Reference) (OtherBodyIndex :type Integer) (bFromSweep :type Boolean) (SweepResult :type Hit%20Result%20Structure%20%28by%20ref%29))
  (bind _asbp_money (Utilities|Casting|CastToBP_Money OtherActor))
  (bind _returnvalue (Utilities|GetDataTableRow "/Game/Inventory/DataTable/DT_Money.DT_Money" (.rowname (Variables|/Game/Inventory/Blueprint/BP_Money.BP_Money_C|GetMoney _asbp_money)))
    (:then
      (Variables|Money|SetMoneyAmountInven (+ (.amount _returnvalue) (Variables|Money|GetMoneyAmountInven)))
      (Actor|DestroyActor _asbp_money)
      ;[1 1 1] Set money amount in WBP inventory with money amount inven(Money amount is bind to money text in designer view)
      (Variables|/Game/Inventory/Widgets/WBP_Inventory.WBP_Inventory_C|SetMoneyAmount (Variables|Widget|GetWBP_Inventory) (Variables|Money|GetMoneyAmountInven))
      (return))))

(fn IncreaseHealth
  (params (HealthToIncrease :type Float%20%28double-precision%29))
  (Variables|HealthBar|SetHealth (+ HealthToIncrease (Variables|HealthBar|GetHealth)))
  ;[1 1 1] Gameplay health bar
  (Default|UpdateHealthBar (Variables|Widget|GetWBP_HealthBar))
  ;[1 1 1] Inventory health bar
  (Default|UpdateHealthBar (Variables|/Game/Inventory/Widgets/WBP_Inventory.WBP_Inventory_C|GetWBP_HealthBar (Variables|Widget|GetWBP_Inventory))))

(fn DecreaseHealth
  (params (HealthToDecrease :type Float%20%28double-precision%29))
  (Variables|HealthBar|SetHealth (- (Variables|HealthBar|GetHealth) HealthToDecrease))
  ;[1 1 1] Gameplay health bar
  (Default|UpdateHealthBar (Variables|Widget|GetWBP_HealthBar))
  ;[1 1 1] Inventory health bar
  (Default|UpdateHealthBar (Variables|/Game/Inventory/Widgets/WBP_Inventory.WBP_Inventory_C|GetWBP_HealthBar (Variables|Widget|GetWBP_Inventory))))

(fn HealthBarInitialization
  (bind _returnvalue (UserInterface|CreateWidget "/Game/Inventory/Widgets/WBP_HealthBar.WBP_HealthBar_C"))
  (bind _output_get (Variables|Widget|SetWBP_HealthBar _returnvalue))
  (Class|UserWidget|SetPositioninViewport _output_get "(X=5.000000,Y=5.000000)" true)
  (UserInterface|Viewport|AddtoViewport _output_get 0))

(fn TraceItemtoPickUp
  (bind _returnvalue (Game|GetPlayerCharacter 0))
  (bind _returnvalue_2 (Transformation|GetActorLocation _returnvalue))
  (bind _returnvalue_3 (- _returnvalue_2 "0.000000,0.000000,60.000000"))
  (bind _outhit (Collision|SphereTraceByChannel _returnvalue_3 (+ _returnvalue_3 (* (Transformation|GetActorForwardVector _returnvalue) 1.5e+02)) 3e+01 "TraceTypeQuery1" false 0 "ForOneFrame"))
  (bind _asbp_item (Utilities|Casting|CastToBP_Item (.hitactor _outhit))
    (:then
      (return (Variables|/Game/Inventory/Blueprint/BP_Item.BP_Item_C|GetItem _asbp_item) true (.hitactor _outhit)))
    (:CastFailed
      (return "" false 0))))

(fn AddtoInventory
  (params (Item :type S%20Slot%20Structure))
  (bind (_itemid _quantity _itemtype) (Utilities|Struct|BreakS_Slot Item))
  (bind (_itemid_2 _quantity_2 _itemtype_2) (Utilities|Struct|BreakS_Slot Item))
  (bind (_itemid_3 _quantity_3) (Utilities|Struct|BreakS_Slot Item))
  (bind (_itemid_4 _quantity_4 _itemtype_3) (Utilities|Struct|BreakS_Slot Item))
  (bind (_itemid_5 _quantity_5) (Utilities|Struct|BreakS_Slot Item))
  (switch Utilities|FlowControl|Switch|SwitchonE_ItemTypes (.ItemType (Utilities|Struct|BreakS_Slot Item))
    (:NewEnumerator0
      (for (_array_element _array_index) (.Swords (Utilities|Struct|BreakS_AllItem (Variables|Default|GetAllItem)))
        (if (== (.RowName (Utilities|Struct|BreakDataTableRowHandle (.ItemID (Utilities|Struct|BreakS_Slot _array_element)))) (.RowName (Utilities|Struct|BreakDataTableRowHandle (.ItemID (Utilities|Struct|BreakS_Slot Item)))))
          (bind _returnvalue (Utilities|GetDataTableRow "/Game/Inventory/DataTable/DT_Items.DT_Items" (.RowName (Utilities|Struct|BreakDataTableRowHandle (.ItemID (Utilities|Struct|BreakS_Slot Item)))))
            (:then
              (if (>= (.StackSize (Utilities|Struct|BreakS_Item _returnvalue)) (+ (.Quantity (Utilities|Struct|BreakS_Slot Item)) (.Quantity (Utilities|Struct|BreakS_Slot _array_element))))
                (Utilities|Array|SetArrayElem (.Swords (Utilities|Struct|BreakS_AllItem (Variables|Default|GetAllItem))) _array_index (Utilities|Struct|MakeS_Slot _itemid_2 (+ (.Quantity (Utilities|Struct|BreakS_Slot Item)) (.Quantity (Utilities|Struct|BreakS_Slot _array_element))) _itemtype_2))
                (return true))))))
      (for (_array_element_2 _array_index_2) (.Swords (Utilities|Struct|BreakS_AllItem (Variables|Default|GetAllItem)))
        (if (== (.Quantity (Utilities|Struct|BreakS_Slot _array_element_2)) 0)
          (Utilities|Array|SetArrayElem (.Swords (Utilities|Struct|BreakS_AllItem (Variables|Default|GetAllItem))) _array_index_2 Item)
          (return true)))
      (return false))
    (:NewEnumerator1
      (for (_array_element_3 _array_index_3) (.Shield (Utilities|Struct|BreakS_AllItem (Variables|Default|GetAllItem)))
        (if (== (.RowName (Utilities|Struct|BreakDataTableRowHandle (.ItemID (Utilities|Struct|BreakS_Slot _array_element_3)))) (.RowName (Utilities|Struct|BreakDataTableRowHandle (.ItemID (Utilities|Struct|BreakS_Slot Item)))))
          (bind _returnvalue_2 (Utilities|GetDataTableRow "/Game/Inventory/DataTable/DT_Items.DT_Items" (.RowName (Utilities|Struct|BreakDataTableRowHandle _itemid_5)))
            (:then
              (if (>= (.StackSize (Utilities|Struct|BreakS_Item _returnvalue_2)) (+ _quantity_5 (.Quantity (Utilities|Struct|BreakS_Slot _array_element_3))))
                ;[1 1 1] update the item array slot
                (Utilities|Array|SetArrayElem (.Shield (Utilities|Struct|BreakS_AllItem (Variables|Default|GetAllItem))) _array_index_3 (Utilities|Struct|MakeS_Slot _itemid (+ _quantity_5 (.Quantity (Utilities|Struct|BreakS_Slot _array_element_3))) _itemtype))
                (return true))))))
      (Development|PrintString "Should make another slot for that item")
      (for (_array_element_4 _array_index_4) (.Shield (Utilities|Struct|BreakS_AllItem (Variables|Default|GetAllItem)))
        (if (== (.Quantity (Utilities|Struct|BreakS_Slot _array_element_4)) 0)
          (Utilities|Array|SetArrayElem (.Shield (Utilities|Struct|BreakS_AllItem (Variables|Default|GetAllItem))) _array_index_4 Item)
          (return true)))
      ;[1 0 0] Fail to add item in inventory
      (Development|PrintString "Failed to add item")
      (return false))
    (:NewEnumerator2
      (for (_array_element_5 _array_index_5) (.Eatable (Utilities|Struct|BreakS_AllItem (Variables|Default|GetAllItem)))
        (if (== (.RowName (Utilities|Struct|BreakDataTableRowHandle (.ItemID (Utilities|Struct|BreakS_Slot _array_element_5)))) (.RowName (Utilities|Struct|BreakDataTableRowHandle (.ItemID (Utilities|Struct|BreakS_Slot Item)))))
          (bind _returnvalue_3 (Utilities|GetDataTableRow "/Game/Inventory/DataTable/DT_Items.DT_Items" (.RowName (Utilities|Struct|BreakDataTableRowHandle _itemid_3)))
            (:then
              (if (>= (.StackSize (Utilities|Struct|BreakS_Item _returnvalue_3)) (+ _quantity_3 (.Quantity (Utilities|Struct|BreakS_Slot _array_element_5))))
                ;[1 1 1] update the item array slot
                (Utilities|Array|SetArrayElem (.Eatable (Utilities|Struct|BreakS_AllItem (Variables|Default|GetAllItem))) _array_index_5 (Utilities|Struct|MakeS_Slot _itemid_4 (+ _quantity_3 (.Quantity (Utilities|Struct|BreakS_Slot _array_element_5))) _itemtype_3))
                (return true))))))
      (Development|PrintString "Should make another slot for that item")
      (for (_array_element_6 _array_index_6) (.Eatable (Utilities|Struct|BreakS_AllItem (Variables|Default|GetAllItem)))
        (if (== (.Quantity (Utilities|Struct|BreakS_Slot _array_element_6)) 0)
          (Utilities|Array|SetArrayElem (.Eatable (Utilities|Struct|BreakS_AllItem (Variables|Default|GetAllItem))) _array_index_6 Item)
          (return true)))
      ;[1 0 0] Fail to add item in inventory
      (Development|PrintString "Failed to add item")
      (return false))))

(fn UpgradeInventory
  (params (SwordSlotsAmount :type Integer) (ShieldSlotsAmount :type Integer) (EatableSlotsAmount :type Integer))
  (bind _allitem (Variables|Default|GetAllItem))
  (bind (_swords _shield _eatable) (Utilities|Struct|BreakS_AllItem _allitem))
  (Utilities|Array|Resize _swords (+ SwordSlotsAmount (Utilities|Array|Length _swords)))
  (Utilities|Array|Resize _shield (+ ShieldSlotsAmount (Utilities|Array|Length _shield)))
  (Utilities|Array|Resize _eatable (+ EatableSlotsAmount (Utilities|Array|Length _eatable)))
  (Default|UpdateItemsinInventoryUI (Variables|Widget|GetWBP_Inventory) (Variables|Default|GetAllItem)))

(fn SetInventorySize
  (params (SwordTabSize :type Integer) (ShieldTabSize :type Integer) (EatableTabSize :type Integer))
  (bind _allitem (Variables|Default|GetAllItem))
  (bind (_swords _shield _eatable) (Utilities|Struct|BreakS_AllItem _allitem))
  (Utilities|Array|Resize _swords SwordTabSize)
  (Utilities|Array|Resize _shield ShieldTabSize)
  (Utilities|Array|Resize _eatable EatableTabSize)
  (Default|UpdateItemsinInventoryUI (Variables|Widget|GetWBP_Inventory) (Variables|Default|GetAllItem)))

(fn DecreaseQuantityOfSpecificItemName
  (params (Item :type S%20Slot%20Structure))
  (bind _allitem (Variables|Default|GetAllItem))
  (bind _swords (Utilities|Struct|BreakS_AllItem _allitem))
  (LocalVariables|SetFound false)
  (for (_array_element _array_index) (.Swords (Utilities|Struct|BreakS_AllItem (Variables|Default|GetAllItem)))
    (if (LocalVariables|GetFound)
      (Development|PrintString "Item ALREADY founded so return this function" true true "(R=0.000000,G=0.660000,B=1.000000,A=1.000000)" 8e+01)
      (return)
      (elif (> (.Quantity (Utilities|Struct|BreakS_Slot _array_element)) 0)
        (Development|PrintString (Utilities|String|ToString(Text) (Utilities|Text|FormatText "index{Index} slot has quantity" _array_index)) true true "(R=1.000000,G=0.027120,B=0.723949,A=1.000000)" 8e+01)
        (if (== (.RowName (Utilities|Struct|BreakDataTableRowHandle (.ItemID (Utilities|Struct|BreakS_Slot _array_element)))) (.RowName (Utilities|Struct|BreakDataTableRowHandle (.ItemID (Utilities|Struct|BreakS_Slot Item)))))
          (Development|PrintString (Utilities|String|ToString(Text) (Utilities|Text|FormatText "Item found at index {Index}" 0)) true true "(R=0.096141,G=1.000000,B=0.298657,A=1.000000)" 8e+01)
          (Utilities|Array|SetArrayElem _swords _array_index (Utilities|Struct|MakeS_Slot (.ItemID (Utilities|Struct|BreakS_Slot (Utilities|Array|Get(acopy) _swords _array_index))) (- (.Quantity (Utilities|Struct|BreakS_Slot (Utilities|Array|Get(acopy) _swords _array_index))) 1) (.ItemType (Utilities|Struct|BreakS_Slot (Utilities|Array|Get(acopy) _swords _array_index)))))
          (LocalVariables|SetFound true)
          (Development|PrintString "Set Found variable TRUE" true true "(R=1.000000,G=0.026601,B=0.000000,A=1.000000)" 8e+01)
          (else
            (Development|PrintString (Utilities|String|ToString(Text) (Utilities|Text|FormatText "Item not found at index{Index}" _array_index)) true true "(R=1.000000,G=0.027120,B=0.723949,A=1.000000)" 8e+01)))))))